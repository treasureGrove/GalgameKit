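; TalkComponent is a player-side component that runs NPC conversations and switches the player between exploration, talking and menu-pause states, adjusting cursor and input mode.
; It creates the HUD on BeginPlay, tracks the NPC passed in by sphere trace and shows its interact prompt.
; Starting dialog blends the camera to the NPC and reads its DataTable by row number.
; Clicks finish typing or advance rows; a missing row ends the talk and restores the camera.
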(event `ClickEvent`
  (bind _wg_dialog (`self.WG Dialog`))
  (if (`/Game/GalGame/UI/GalPlayHUD/WG_Dialog.IsTyping?` _wg_dialog)
    (`/Game/GalGame/UI/GalPlayHUD/WG_Dialog.EndLine` _wg_dialog)
    (else
      (`self.NextRow`)
      (`self.SetRow`))))

(event `self.ReceiveBeginPlay`
  (bind _returnvalue (`|CreateWidget` "/Game/GalGame/UI/GalPlayHUD/WG_HUD.WG_HUD_C"))
  (bind _output_get (set `self.HUD` _returnvalue))
  (`UserWidget.AddToViewport` _output_get 0)
  (bind _wg_dialog (`/Game/GalGame/UI/GalPlayHUD/WG_HUD.WG_Dialog` _output_get))
  (set `self.WG Dialog` _wg_dialog)
  (set `self.DialogText` (`/Game/GalGame/UI/GalPlayHUD/WG_Dialog.RichDialogText` _wg_dialog))
  (set `self.Name` (`/Game/GalGame/UI/GalPlayHUD/WG_Dialog.Name` _wg_dialog))
  (set `self.Character Face` (`/Game/GalGame/UI/GalPlayHUD/WG_Dialog.CharacterFace` _wg_dialog))
  (`Widget.SetVisibility` (`/Game/GalGame/UI/GalPlayHUD/WG_HUD.WG_Dialog` _output_get) "Hidden")
  (`Widget.SetVisibility` (`/Game/GalGame/UI/GalPlayHUD/WG_HUD.WG_GameMenu` _output_get) "Hidden"))

(event `Key|One`
  (params (Key :type "Key Structure"))
  (:`Pressed`
    (`self.SetRow`)))

(fn `HiddenDIalogUI`
  (bind _wg_dialog (`/Game/GalGame/UI/GalPlayHUD/WG_HUD.WG_Dialog` (`self.HUD`)))
  (`UserWidget.PlayAnimation` _wg_dialog (`/Game/GalGame/UI/GalPlayHUD/WG_Dialog.FadeOut` _wg_dialog) 0.0 1 "Forward" 1.0 false))

(fn `LeaveNpc`
  (params (OtherActor :type "Actor Object Reference"))
  (bind _currentnpc (`self.CurrentNPC`))
  (`/Engine/EditorBlueprintResources/StandardMacros.IsValid` _currentnpc
    (:`Is Valid`
      (`SceneComponent.SetHiddenInGame` (`/Game/GalGame/Blueprints/NPC/BP_NPC.InteractMessage` _currentnpc) true false)
      (set `/Game/GalGame/Blueprints/NPC/BP_NPC.IsTalking` false _currentnpc)
      (set `self.IsTalking` false)
      (if true
        (set `self.CurrentNPC` null)
        (set `self.TalkingNPC` "")
        (`self.SetPlayerState` "NewEnumerator0")
        (`self.HiddenDIalogUI`)
        (`PlayerController.SetViewTargetWithBlend` (`self.Player Controller`) (`self.Character`) 0.5 "VTBlend_Cubic" 0.0 false)
        (else
          (`KismetSystemLibrary.PrintString` "Failed"))))))

(fn `NextRow`
  (switch `/Game/GalGame/Blueprints/Enums/E_PlayerStates` (`self.PlayerState`)
    (:`NewEnumerator1`
      (`/Engine/EditorBlueprintResources/StandardMacros.IsValid` (`self.CurrentDialogDatas`)
        (:`Is Valid`
          (set `self.CurrentRow` (+ (`self.CurrentRow`) 1)))
        (:`Is Not Valid`
          (`self.LeaveNpc` null))))))

(fn `SetInitializeReference`
  (params (Camera :type "CameraComponent Object Reference") (PlayerController :type "PlayerController Object Reference") (Character :type "Character Object Reference") (Sphere :type "SphereComponent Object Reference"))
  (returns (Return :type Boolean))
  (set `self.Camera` Camera)
  (set `self.Player Controller` PlayerController)
  (set `self.Character` Character)
  (set `self.Sphere` Sphere)
  (`self.Player Controller`
    (:`then`
      (return false))
    (:`else`
      (set `self.Player Controller` (`GameplayStatics.GetPlayerController` 0))
      (return false))))

(fn `SetPlayerState`
  (params (PlayerState :type "/Game/GalGame/Blueprints/Enums/E_PlayerStates Enum" :default "NewEnumerator0"))
  (bind _player_controller (`self.Player Controller`))
  (bind _output_get (set `self.PlayerState` PlayerState))
  (switch `/Game/GalGame/Blueprints/Enums/E_PlayerStates` _output_get
    (:`NewEnumerator0`
      (set `PlayerController.bShowMouseCursor` false (`self.Player Controller`))
      (`WidgetBlueprintLibrary.SetInputMode_GameOnly` _player_controller))
    (:`NewEnumerator1`
      (set `PlayerController.bShowMouseCursor` true (`self.Player Controller`))
      (`WidgetBlueprintLibrary.SetInputMode_GameAndUIEx` _player_controller null))
    (:`NewEnumerator3`
      (set `PlayerController.bShowMouseCursor` true (`GameplayStatics.GetPlayerController` 0))
      (`WidgetBlueprintLibrary.SetInputMode_GameAndUIEx` (`GameplayStatics.GetPlayerController` 0) null))))

(fn `SetRow`
  (bind _currentdialogdatas (`self.CurrentDialogDatas`))
  (`/Engine/EditorBlueprintResources/StandardMacros.IsValid` _currentdialogdatas
    (:`Is Valid`
      (bind _returnvalue (`|GetDataTableRow` _currentdialogdatas (`KismetStringLibrary.Conv_StringToName` (`KismetStringLibrary.Conv_IntToString` (+ (`self.CurrentRow`) 1))))
        (:`then`
          (bind (_name _expression _dialog _bgm _soundeffect _voice _background _characterposition _effects _characterface) (break `/Game/GalGame/Blueprints/Structures/Legacy/ST_Dialog_legacy` _returnvalue))
          (`TextBlock.SetText` (`self.Name`) (`KismetTextLibrary.Conv_StringToText` (`|GetEnumeratorNameAsString` _name)))
          ;[1 0.8782 0.278] 换角色位置
          (`/Game/GalGame/UI/GalPlayHUD/WG_Dialog.TypeText` (`self.WG Dialog`) _dialog)
          (set `self.FullString` _dialog)
          (`/Engine/EditorBlueprintResources/StandardMacros.IsValid` _characterface
            (:`Is Valid`
              (`Image.SetBrushFromTexture` (`self.Character Face`) _characterface false))))
        (:`RowNotFound`
          (`KismetSystemLibrary.PrintString` "GetRowFaild")
          (`self.LeaveNpc` null))))))

(fn `ShowDialogUI`
  (bind _wg_dialog (`/Game/GalGame/UI/GalPlayHUD/WG_HUD.WG_Dialog` (`self.HUD`)))
  (`Widget.SetVisibility` _wg_dialog "Visible")
  (`UserWidget.PlayAnimation` _wg_dialog (`/Game/GalGame/UI/GalPlayHUD/WG_Dialog.FadeIn` _wg_dialog) 0.0 1 "Forward" 1.0 false))

(fn `ShowMenuUI`
  (bind _wg_gamemenu (`/Game/GalGame/UI/GalPlayHUD/WG_HUD.WG_GameMenu` (`self.HUD`)))
  (if (`|EnumEquality` (`self.PlayerState`) "NewEnumerator0")
    (`self.SetPlayerState` "NewEnumerator3")
    (`Widget.SetVisibility` _wg_gamemenu "Visible")
    (else
      (`self.SetPlayerState` "NewEnumerator0")
      (`Widget.SetVisibility` _wg_gamemenu "Hidden")
      (`KismetSystemLibrary.PrintString` "B"))))

(fn `SphereTraceNpc`
  (params (OtherActor :type "Actor Object Reference"))
  ;[1 1 1] 获取NPC
  (bind _asbp_npc (cast `/Game/GalGame/Blueprints/NPC/BP_NPC` OtherActor))
  (bind _output_get (set `self.CurrentNPC` _asbp_npc))
  (set `self.TalkingNPC` (`/Game/GalGame/Blueprints/NPC/BP_NPC.MyName` _asbp_npc))
  (`SceneComponent.SetHiddenInGame` (`/Game/GalGame/Blueprints/NPC/BP_NPC.InteractMessage` _output_get) false false))

(fn `StartDialog`
  (bind _currentnpc (`self.CurrentNPC`))
  (if (not (`self.IsTalking`))
    ;[1 1 1] 注视玩家，并锁定输入
    (`self.SetPlayerState` "NewEnumerator1")
    (`/Game/GalGame/Blueprints/NPC/BP_NPC.StartTalk` _currentnpc)
    (`PlayerController.SetViewTargetWithBlend` (`GameplayStatics.GetPlayerController` 0) _currentnpc 0.5 "VTBlend_Cubic" 0.0 false)
    (set `self.CurrentDialogDatas` (`/Game/GalGame/Blueprints/NPC/BP_NPC.DialogData` _currentnpc))
    (set `self.CurrentRow` 0)
    (`self.SetRow`)
    (`self.ShowDialogUI`)
    (set `self.IsTalking` true)))