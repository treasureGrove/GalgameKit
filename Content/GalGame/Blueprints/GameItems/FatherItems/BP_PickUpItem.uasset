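; BP_PickUpItem is a pickup item actor that shows a widget while something overlaps its trigger and can be picked up through interaction.
; The widget is hidden at BeginPlay and toggled by the trigger's begin and end overlap events, with no filtering of the overlapping actor.
; Interact prints a debug message, calls DestoryItem to destroy the actor after a brief delay, and returns the item's static mesh to the caller.
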(event `self.ReceiveBeginPlay`
  (`SceneComponent.SetHiddenInGame` (`self.Widget`) true false))

(event `self.trigger.OnComponentBeginOverlap`
  (params (OverlappedComponent :type "PrimitiveComponent Object Reference") (OtherActor :type "Actor Object Reference") (OtherComp :type "PrimitiveComponent Object Reference") (OtherBodyIndex :type Integer) (bFromSweep :type Boolean) (SweepResult :type "HitResult Structure (by ref)"))
  (`SceneComponent.SetHiddenInGame` (`self.Widget`) false false))

(event `self.trigger.OnComponentEndOverlap`
  (params (OverlappedComponent :type "PrimitiveComponent Object Reference") (OtherActor :type "Actor Object Reference") (OtherComp :type "PrimitiveComponent Object Reference") (OtherBodyIndex :type Integer))
  (`SceneComponent.SetHiddenInGame` (`self.Widget`) true false))

(event `DestoryItem`
  (`KismetSystemLibrary.Delay` 0.02)
  (`self.K2_DestroyActor`))

(fn `Interact`
  (returns (StaticMesh :type "StaticMesh Object Reference"))
  (`KismetSystemLibrary.PrintString` "PickedUp")
  (`self.DestoryItem`)
  (return (`StaticMeshComponent.StaticMesh` (`self.ItemMesh`))))

(fn `UserConstructionScript`)