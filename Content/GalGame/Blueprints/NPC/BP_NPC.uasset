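; BP_NPC is a visual-novel dialogue NPC, drawn as a textured mesh with front, side and back views chosen by player angle.
; It spawns and slides in other NPCs to either side, registering each in a name-keyed map.
; Name-keyed events drive expressions, dialogue audio and sound effects on those characters.
; Expressions animate material opacity around texture swaps, or play a looping MediaSource through a runtime-created MediaTexture as "Live2D".
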(event `self.ReceiveBeginPlay`
  (bind _returnvalue (`GameplayStatics.GetActorOfClass` "/Game/GalGame/Blueprints/Player/BP_Player.BP_Player_C"))
  (set `self.Player` _returnvalue)
  (`SceneComponent.SetHiddenInGame` (`self.InteractMessage`) true false))

(event `self.ReceiveTick`
  (params (DeltaSeconds :type "Float (single-precision)")))

(event `AddCharacterLeft`
  (params (NPC :type "Object Soft Class Reference"))
  (bind _mesh (`self.Mesh`))
  (bind _returnvalue (`SceneComponent.GetRightVector` _mesh))
  ; Comment
  (bind _returnvalue_2 (`KismetSystemLibrary.LoadClassAsset_Blocking` NPC))
  (bind _asbp_npc (castclass `/Game/GalGame/Blueprints/NPC/BP_NPC` _returnvalue_2)
    (:`then`
      (bind _returnvalue_3 (`|SpawnActorFromClass` _asbp_npc (`KismetMathLibrary.MakeTransform` (+ (* _returnvalue 320.0) (`SceneComponent.K2_GetComponentLocation` _mesh) (* _returnvalue 100.0 (`self.LeftNpcIndex`))) (`self.K2_GetActorRotation`)) "Undefined" "MultiplyWithRoot" null null))
      (if (`.ReturnValue` (`BlueprintMapLibrary.Map_Find` (`self.AllTalkingNpc`) (`/Game/GalGame/Blueprints/NPC/BP_NPC.MyName` _returnvalue_3)))
        (`self.K2_DestroyActor` _returnvalue_3)
        (`KismetSystemLibrary.PrintString` "添加角色重复")
        (else
          (`BlueprintMapLibrary.Map_Add` (`self.AllTalkingNpc`) (`/Game/GalGame/Blueprints/NPC/BP_NPC.MyName` _returnvalue_3) _returnvalue_3)
          (bind _rootcomponent (`Actor.RootComponent` _returnvalue_3))
          (bind (_returnvalue_location _returnvalue_rotation) (`KismetMathLibrary.BreakTransform` (`SceneComponent.GetRelativeTransform` _rootcomponent)))
          (`KismetSystemLibrary.MoveComponentTo` _rootcomponent (+ _returnvalue_location (0.0 200.0 0.0)) _returnvalue_rotation true true 0.5)
          (`/Engine/EditorBlueprintResources/StandardMacros.IncrementInt` (`self.LeftNpcIndex`)))))
    (:`CastFailed`
      (`KismetSystemLibrary.PrintString` "AddCharacter类型错误"))))

(event `AddCharacterRight`
  (params (Npc :type "Object Soft Class Reference"))
  (bind _mesh (`self.Mesh`))
  (bind _returnvalue (`SceneComponent.GetRightVector` _mesh))
  ; Comment
  (bind _returnvalue_2 (`KismetSystemLibrary.LoadClassAsset_Blocking` Npc))
  (bind _asbp_npc (castclass `/Game/GalGame/Blueprints/NPC/BP_NPC` _returnvalue_2)
    (:`then`
      (bind _returnvalue_3 (`|SpawnActorFromClass` _asbp_npc (`KismetMathLibrary.MakeTransform` (+ (* _returnvalue -320.0) (`SceneComponent.K2_GetComponentLocation` _mesh) (* _returnvalue -100.0 (`self.RightNpcIndex`))) (`self.K2_GetActorRotation`)) "Undefined" "MultiplyWithRoot" null null))
      (if (`.ReturnValue` (`BlueprintMapLibrary.Map_Find` (`self.AllTalkingNpc`) (`/Game/GalGame/Blueprints/NPC/BP_NPC.MyName` _returnvalue_3)))
        (`self.K2_DestroyActor` _returnvalue_3)
        (`KismetSystemLibrary.PrintString` "添加角色重复")
        (else
          (`BlueprintMapLibrary.Map_Add` (`self.AllTalkingNpc`) (`/Game/GalGame/Blueprints/NPC/BP_NPC.MyName` _returnvalue_3) _returnvalue_3)
          (bind _rootcomponent (`Actor.RootComponent` _returnvalue_3))
          (bind (_returnvalue_location _returnvalue_rotation) (`KismetMathLibrary.BreakTransform` (`SceneComponent.GetRelativeTransform` _rootcomponent)))
          (`KismetSystemLibrary.MoveComponentTo` _rootcomponent (+ _returnvalue_location (0.0 -200.0 0.0)) _returnvalue_rotation true true 0.5)
          (`/Engine/EditorBlueprintResources/StandardMacros.IncrementInt` (`self.RightNpcIndex`)))))
    (:`CastFailed`
      (`KismetSystemLibrary.PrintString` "AddCharacter类型错误"))))

(event `SetExpression`
  (params (Image :type "Map of String to Object Soft Object Reference"))
  (bind _mediaplayer (`self.MediaPlayer`))
  ; 已完成
  (bind _keys (`BlueprintMapLibrary.Map_Keys` Image))
  (for _array_element _keys
    (bind (_value _returnvalue) (`BlueprintMapLibrary.Map_Find` Image _array_element))
    (if _returnvalue
      (`/Engine/EditorBlueprintResources/StandardMacros.IsValid` (`self.GetNPCByName` _array_element)
        (:`Is Valid`
          (bind _returnvalue_2 (`KismetSystemLibrary.LoadAsset_Blocking` _value))
          (bind _astexture (cast `Texture` _returnvalue_2)
            (:`then`
              (bind (_direction _opacity) (`Timeline|Timeline` :!via `PlayFromStart`)
                (:`Update`
                  (bind _currentmaterial (`/Game/GalGame/Blueprints/NPC/BP_NPC.CurrentMaterial` (`self.GetNPCByName` _array_element)))
                  (`MaterialInstanceDynamic.SetScalarParameterValue` _currentmaterial "Opacity" _opacity))
                (:`Finished`
                  (`MaterialInstanceDynamic.SetTextureParameterValue` (`/Game/GalGame/Blueprints/NPC/BP_NPC.CurrentMaterial` (`self.GetNPCByName` _array_element)) "CharacterShows" _astexture)
                  (bind (_direction_2 _opacity_2) (`Timeline|Timeline_0` :!via `PlayFromStart`)
                    (:`Update`
                      (`MaterialInstanceDynamic.SetScalarParameterValue` (`/Game/GalGame/Blueprints/NPC/BP_NPC.CurrentMaterial` (`self.GetNPCByName` _array_element)) "Opacity" _opacity_2))))))
            (:`CastFailed`
              (bind _asmedia_source (cast `MediaSource` _returnvalue_2))
              (`MediaPlayer.OpenSource` _mediaplayer _asmedia_source)
              (`MediaPlayer.SetLooping` _mediaplayer true)
              (`MediaPlayer.Play` _mediaplayer)
              (`MediaTexture.SetMediaPlayer` (`self.Live2DTexture`) _mediaplayer)
              (`KismetSystemLibrary.Delay` 0.1)
              (`MaterialInstanceDynamic.SetTextureParameterValue` _currentmaterial "CharacterShows" (`self.Live2DTexture`))
              (bind (_direction_3 _opacity_3) (`Timeline|Timeline_2` :!via `PlayFromStart`)
                (:`Update`
                  (`MaterialInstanceDynamic.SetScalarParameterValue` _currentmaterial "Opacity" _opacity_3))))))
        (:`Is Not Valid`
          (`KismetSystemLibrary.PrintString` "NoSuchName")))
      (else
        (`KismetSystemLibrary.PrintString` "NoSuchName")))))

(event `SetDialogSound`
  (params (DialogSound :type "Map of String to SoundCue Object Reference"))
  ;[1 0.7434 0 0.5] Comment
  (bind _keys (`BlueprintMapLibrary.Map_Keys` DialogSound))
  (for _array_element _keys
    (bind (_value _returnvalue) (`BlueprintMapLibrary.Map_Find` DialogSound _array_element))
    (if _returnvalue
      (bind _value_2 (`self.GetNPCByName` _array_element))
      (`/Engine/EditorBlueprintResources/StandardMacros.IsValid` _value_2
        (:`Is Valid`
          (bind _audio (`/Game/GalGame/Blueprints/NPC/BP_NPC.Audio` _value_2))
          (`AudioComponent.SetSound` _audio _value)
          (`AudioComponent.Play` _audio 0.0)))
      (else
        (`KismetSystemLibrary.PrintString` "NoSuchSound")))))

(event `self.Audio.OnAudioFinished`)

(event `PlaySoundEffect`
  (params (Sounds :type "Map of String to Object Soft Object Reference"))
  (bind _keys (`BlueprintMapLibrary.Map_Keys` Sounds))
  (for _array_element _keys
    (bind (_value _returnvalue) (`BlueprintMapLibrary.Map_Find` Sounds _array_element))
    (if _returnvalue
      (bind _returnvalue_2 (`KismetSystemLibrary.LoadAsset_Blocking` _value))
      (bind _assound_cue (cast `SoundCue` _returnvalue_2))
      (`GameplayStatics.PlaySoundAtLocation` _assound_cue (`self.K2_GetActorLocation` (`self.GetNPCByName` _array_element)) (struct) 1.0 1.0 0.0 null null null null))))

(fn `GetDataTable`
  (returns (TalkingDatas :type "DataTable Object Reference"))
  (return (`self.TalkingData`)))

(fn `GetMaterial`
  (bind _returnvalue (`PrimitiveComponent.CreateDynamicMaterialInstance` (`self.Mesh`) 0 (`PrimitiveComponent.GetMaterial` (`self.Mesh`) 0) "None"))
  (bind _output_get (set `self.CurrentMaterial` _returnvalue))
  (`PrimitiveComponent.SetMaterial` (`self.Mesh`) 0 _output_get)
  (`MaterialInstanceDynamic.SetTextureParameterValue` (`self.CurrentMaterial`) "CharacterShows" (`self.FrontTexture`)))

(fn `GetNPCByName`
  (params (Key :type String))
  (returns (Value :type "/Game/GalGame/Blueprints/NPC/BP_NPC Object Reference"))
  (bind (_value _returnvalue) (`BlueprintMapLibrary.Map_Find` (`self.AllTalkingNpc`) Key))
  (if _returnvalue
    (return _value)
    (else
      (`KismetSystemLibrary.PrintString` "没有对应的角色名或输入角色名为错误")
      (return null))))

(fn `LetJump`
  (returns (ReturnValue :type Boolean))
  (`self.Jump`)
  (return false))

(fn `StartTalk`
  (set `self.IsTalking` true)
  (`MaterialInstanceDynamic.SetTextureParameterValue` (`self.CurrentMaterial`) "CharacterShows" (`self.FrontTexture`))
  (`SceneComponent.K2_SetRelativeRotation` :`self` (`self.Mesh`)))

(fn `StopAllDialogSound`
  (bind _alltalkingnpc (`self.AllTalkingNpc`))
  (bind _keys (`BlueprintMapLibrary.Map_Keys` _alltalkingnpc))
  (for _array_element _keys
    (bind (_value _returnvalue) (`BlueprintMapLibrary.Map_Find` _alltalkingnpc _array_element))
    (if _returnvalue
      (`AudioComponent.Stop` (`/Game/GalGame/Blueprints/NPC/BP_NPC.Audio` _value)))))

(fn `UpdateCharacterFace`
  (bind _returnvalue (`KismetMathLibrary.DegAcos` (`KismetMathLibrary.Vector_CosineAngle2D` (`self.GetActorForwardVector`) (`KismetMathLibrary.Normal` (- (`self.K2_GetActorLocation` (`GameplayStatics.GetPlayerPawn` 0)) (`self.K2_GetActorLocation`))))))
  (if (`self.IsTalking`)
    _
    (elif (`KismetMathLibrary.InRange_FloatFloat` _returnvalue 0.0 65.0)
      (`MaterialInstanceDynamic.SetTextureParameterValue` (`self.CurrentMaterial`) "CharacterShows" (`self.FrontTexture`))
      (`SceneComponent.K2_SetRelativeRotation` :`self` (`self.Mesh`))
      (elif (`KismetMathLibrary.InRange_FloatFloat` _returnvalue 65.0 115.0 false)
        (`MaterialInstanceDynamic.SetTextureParameterValue` (`self.CurrentMaterial`) "CharacterShows" (`self.SideTexture`))
        (`SceneComponent.K2_SetRelativeRotation` (`self.Mesh`) (struct :`Yaw` 90.0) false false)
        (else
          (`MaterialInstanceDynamic.SetTextureParameterValue` (`self.CurrentMaterial`) "CharacterShows" (`self.BackTexture`))
          (`SceneComponent.K2_SetRelativeRotation` :`self` (`self.Mesh`)))))))

(fn `UserConstructionScript`
  (`self.GetMaterial`)
  (`BlueprintMapLibrary.Map_Add` (`self.AllTalkingNpc`) "CurrentNpc" self)
  (`BlueprintMapLibrary.Map_Add` (`self.AllTalkingNpc`) (`self.MyName`) self)
  (`BlueprintMapLibrary.Map_Add` (`self.AllTalkingNpc`) "" self)
  (bind _returnvalue (`|GenericCreateObject` "/Script/MediaAssets.MediaPlayer"))
  (set `self.MediaPlayer` _returnvalue)
  (bind _returnvalue_2 (`|GenericCreateObject` "/Script/MediaAssets.MediaTexture"))
  (set `self.Live2DTexture` _returnvalue_2)
  (`MediaTexture.SetMediaPlayer` (`self.Live2DTexture`) (`self.MediaPlayer`))
  (set `self.RightNpcIndex` 0)
  (set `self.LeftNpcIndex` 0))