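; NPC base with a flat, Doom-style directional look that shows a front, side or back texture depending on where the player stands.
; Construction creates a dynamic material on the mesh, and BeginPlay hides the interact message and starts a fast looping timer.
; The timer compares the actor's forward vector with the 2D direction to the player, swapping texture and turning the mesh for side views.
; StartTalk locks the front view.
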(event `self.ReceiveBeginPlay`
  (`KismetSystemLibrary.K2_SetTimerDelegate` (delegate `CharacterFace`) 0.05 true)
  (bind _returnvalue (`GameplayStatics.GetActorOfClass` "/Game/Blueprints/Player/BP_Player.BP_Player_C"))
  (set `self.Player` _returnvalue)
  (`SceneComponent.SetHiddenInGame` (`self.InteractMessage`) true false))

(event `CharacterFace`
  (`self.UpdateCharacterFace`))

(event `self.ReceiveTick`
  (params (DeltaSeconds :type "Float (single-precision)")))

(fn `GetMaterial`
  (bind _returnvalue (`PrimitiveComponent.CreateDynamicMaterialInstance` (`self.Mesh`) 0 (`PrimitiveComponent.GetMaterial` (`self.Mesh`) 0) "None"))
  (bind _output_get (set `self.CurrentMaterial` _returnvalue))
  (`PrimitiveComponent.SetMaterial` (`self.Mesh`) 0 _output_get)
  (`MaterialInstanceDynamic.SetTextureParameterValue` (`self.CurrentMaterial`) "CharacterShows" (`self.FrontTexture`)))

(fn `StartTalk`
  (set `self.IsTalking` true)
  (`MaterialInstanceDynamic.SetTextureParameterValue` (`self.CurrentMaterial`) "CharacterShows" (`self.FrontTexture`))
  (`SceneComponent.K2_SetRelativeRotation` :`self` (`self.Mesh`)))

(fn `UpdateCharacterFace`
  (bind _returnvalue (`KismetMathLibrary.DegAcos` (`KismetMathLibrary.Vector_CosineAngle2D` (`self.GetActorForwardVector`) (`KismetMathLibrary.Normal` (- (`self.K2_GetActorLocation` (`GameplayStatics.GetPlayerPawn` 0)) (`self.K2_GetActorLocation`))))))
  (if (`self.IsTalking`)
    _
    (elif (`KismetMathLibrary.InRange_FloatFloat` _returnvalue 0.0 65.0)
      (`MaterialInstanceDynamic.SetTextureParameterValue` (`self.CurrentMaterial`) "CharacterShows" (`self.FrontTexture`))
      (`SceneComponent.K2_SetRelativeRotation` :`self` (`self.Mesh`))
      (elif (`KismetMathLibrary.InRange_FloatFloat` _returnvalue 65.0 115.0 false)
        (`MaterialInstanceDynamic.SetTextureParameterValue` (`self.CurrentMaterial`) "CharacterShows" (`self.SideTexture`))
        (`SceneComponent.K2_SetRelativeRotation` (`self.Mesh`) (struct :`Yaw` 90.0) false false)
        (else
          (`MaterialInstanceDynamic.SetTextureParameterValue` (`self.CurrentMaterial`) "CharacterShows" (`self.BackTexture`))
          (`SceneComponent.K2_SetRelativeRotation` :`self` (`self.Mesh`)))))))

(fn `UserConstructionScript`
  (`self.GetMaterial`))